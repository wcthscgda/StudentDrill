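; Day/night cycle Blueprint for the main menu sky, rotating a Sun actor over a configurable day length in minutes.
; BeginPlay derives seconds per game hour; Tick advances Hour, converts it to sun pitch and refreshes SkyDome's sun direction.
; Tick also sets NightTime true whenever the truncated Hour is 6 or above, false below.
; Hour is never wrapped in this graph, so NightTime stays true once it reaches 6.
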(event EventBeginPlay
  (bind _output_get (Variables|Default|SetOne%20Day (* (Variables|Default|GetDay%20Length%20in%20Minutes) 6e+01)))
  (Variables|Default|SetOne%20Hour (/ _output_get 24.0)))

(event EventTick
  (params (DeltaSeconds :type Float%20%28single-precision%29))
  (Utilities|FlowControl|Sequence
    (:then_0
      (bind _output_get (Variables|Default|SetHour (+ (Variables|Default|GetHour) (/ DeltaSeconds (Variables|Default|GetOne%20Hour)))))
      (bind _output_get_2 (Variables|Default|SetSun%20Angle (+ (* (/ _output_get 6.0) 9e+01) 9e+01)))
      (Transformation|SetActorRotation (Variables|Default|GetSun) (Math|Rotator|MakeRotator 0.0 _output_get_2 0.0))
      (Default|UpdateSunDirection (Variables|Default|GetSky%20Dome)))
    (:then_1
      (Math|Integer|CompareInt (Math|Float|Truncate (Variables|Default|GetHour)) 6
        (:>
          (Variables|Default|SetNightTime true :!label _label))
        (:==
          (goto _label))
        (:<
          (Variables|Default|SetNightTime false))))))

(fn ConstructionScript)