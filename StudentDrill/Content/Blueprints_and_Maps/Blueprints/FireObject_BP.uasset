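; FireObject_BP is a fire actor that spreads to nearby flammable objects and is destroyed when a ThirdPersonCharacter overlaps its sphere.
; On BeginPlay, it waits briefly, then makes a single pass over its overlapping actors for the "Flamable" tag.
; Each match loses the tag, preventing re-ignition, and gets a new FireObject_BP spawned at its location, creating a self-propagating chain.
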(event OnComponentBeginOverlap(Sphere)
  (params (OverlappedComponent :type Primitive%20Component%20Object%20Reference) (OtherActor :type Actor%20Object%20Reference) (OtherComp :type Primitive%20Component%20Object%20Reference) (OtherBodyIndex :type Integer) (bFromSweep :type Boolean) (SweepResult :type Hit%20Result%20Structure%20%28by%20ref%29))
  (Utilities|Casting|CastToThirdPersonCharacter OtherActor)
  (Actor|DestroyActor))

(event Custom|SpreadFire
  (Utilities|FlowControl|Delay 2.0)
  (for _array_element (Collision|GetOverlappingActors 0 :!class /Script/Engine.Actor)
    (if (Actor|ActorHasTag _array_element "Flamable")
      (Utilities|Array|RemoveItem (Variables|/Script/Engine.Actor|GetTags _array_element) "Flamable")
      (Game|SpawnActorfromClass "FireObject_BP_C" (Math|Conversions|ToTransform(Vector) (Transformation|GetWorldLocation (Variables|/Script/Engine.Actor|GetRootComponent _array_element))) "Undefined" 0 0))))

(event EventBeginPlay
  (CallFunction|SpreadFire))

(fn ConstructionScript)